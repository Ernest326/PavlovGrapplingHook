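; Grappling gun custom item that lets the holding character pull and swing toward whatever it hits.
; On use, a sphere trace from the barrel spawns an attach actor at the hit, parents it to the hit actor and links the cable.
; Hits on another player's hook snap to it.
; While connected, Tick uses LaunchCharacter to counter radial velocity and add pull; release or drop destroys the anchor.
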(event Custom|Set%20Grapple%20Visibility
  (params (NewHidden :type Boolean))
  ;[1 1 1] Change Grapple Visibility
  (Development|SetHiddeninGame (Variables|Default|GetCable) NewHidden false))

(event Custom|Test
  (bind _barell (Variables|Default|GetBarell))
  (bind _returnvalue (Transformation|GetWorldLocation _barell))
  ;[1 1 1] Raycast and check if the grappling gun can be attached to object
  (bind (_outhit _returnvalue_2) (Collision|SphereTraceByChannel _returnvalue (+ _returnvalue (* (Math|Vector|GetForwardVector _barell) (Variables|Settings|GetGrapplingHookLength))) 14.0 "TraceTypeQuery1" false 0 "None"))
  (if _returnvalue_2
    (bind _output_get (Variables|Default|SetHitLocation (.Location (Collision|BreakHitResult _outhit))))
    (bind _returnvalue_3 (Game|SpawnActorfromClass "/Game/CustomMaps/GrapplingHook-v1-0/Blueprints/GrapplingHookAttach.GrapplingHookAttach_C" (Math|Conversions|ToTransform(Vector) _output_get) "AlwaysSpawn" 0 0))
    (Variables|Default|SetGrapplingHookAttach _returnvalue_3)
    (bind _asgrappling_hook (Utilities|Casting|CastToGrapplingHook (.HitActor (Collision|BreakHitResult _outhit)))
      (:then
        (bind _pawn (Class|PavlovCustomItem|GetOwningPawn))
        (if (CallFunction|CanbeGrappeled? _asgrappling_hook (Variables|/Script/Engine.Pawn|GetPlayerState _pawn))
          (Transformation|AttachActorToActor _returnvalue_3 (.HitActor (Collision|BreakHitResult _outhit)) "None" "SnapToTarget" "SnapToTarget" "KeepRelative" true)))
      (:CastFailed
        (Transformation|AttachActorToActor _returnvalue_3 (.HitActor (Collision|BreakHitResult _outhit)) "None" "KeepWorld" "KeepWorld" "KeepWorld" true)))
    (Variables|Default|SetHookConnected true)
    (CallFunction|SetGrappleVisibility false)
    (Class|CableComponent|SetAttachEndto (Variables|Default|GetCable) (Variables|Default|GetGrapplingHookAttach) "None" "None")))

(event EventOnDrop
  ;[1 1 1] Detach the hook when the grappling gun is detached or when you let go of trigger
  (Variables|Default|SetHookConnected false)
  (CallFunction|SetGrappleVisibility true)
  (Actor|DestroyActor (Variables|Default|GetGrapplingHookAttach)))

(event EventOnUse
  (bind _barell (Variables|Default|GetBarell))
  (bind _returnvalue (Transformation|GetWorldLocation _barell))
  ;[1 1 1] Raycast and check if the grappling gun can be attached to object
  (bind (_outhit _returnvalue_2) (Collision|SphereTraceByChannel _returnvalue (+ _returnvalue (* (Math|Vector|GetForwardVector _barell) (Variables|Settings|GetGrapplingHookLength))) 14.0 "TraceTypeQuery1" false 0 "None"))
  (if _returnvalue_2
    (bind _output_get (Variables|Default|SetHitLocation (.Location (Collision|BreakHitResult _outhit))))
    (bind _returnvalue_3 (Game|SpawnActorfromClass "/Game/CustomMaps/GrapplingHook-v1-0/Blueprints/GrapplingHookAttach.GrapplingHookAttach_C" (Math|Conversions|ToTransform(Vector) _output_get) "AlwaysSpawn" 0 0))
    (Variables|Default|SetGrapplingHookAttach _returnvalue_3)
    (bind _asgrappling_hook (Utilities|Casting|CastToGrapplingHook (.HitActor (Collision|BreakHitResult _outhit)))
      (:then
        (bind _pawn (Class|PavlovCustomItem|GetOwningPawn))
        (if (CallFunction|CanbeGrappeled? _asgrappling_hook (Variables|/Script/Engine.Pawn|GetPlayerState _pawn))
          (Transformation|AttachActorToActor _returnvalue_3 (.HitActor (Collision|BreakHitResult _outhit)) "None" "SnapToTarget" "SnapToTarget" "KeepRelative" true)))
      (:CastFailed
        (Transformation|AttachActorToActor _returnvalue_3 (.HitActor (Collision|BreakHitResult _outhit)) "None" "KeepWorld" "KeepWorld" "KeepWorld" true)))
    (Variables|Default|SetHookConnected true)
    (CallFunction|SetGrappleVisibility false)
    (Class|CableComponent|SetAttachEndto (Variables|Default|GetCable) (Variables|Default|GetGrapplingHookAttach) "None" "None")))

(event EventOnUsed
  (params (bJustPicked :type Boolean))
  ;[1 1 1] Detach the hook when the grappling gun is detached or when you let go of trigger
  (Variables|Default|SetHookConnected false)
  (CallFunction|SetGrappleVisibility true)
  (Actor|DestroyActor (Variables|Default|GetGrapplingHookAttach)))

(event EventTick
  (params (DeltaSeconds :type Float%20%28single-precision%29))
  (bind _grapplinghookattach (Variables|Default|GetGrapplingHookAttach))
  ;[1 1 1] Pull and Swing
  (if (Variables|Default|GetHookConnected)
    (bind _pawn (Class|PavlovCustomItem|GetOwningPawn))
    (bind _ascharacter (Utilities|Casting|CastToCharacter _pawn))
    (Character|LaunchCharacter _ascharacter (* (* (* (Math|Vector|Normalize (- (Transformation|GetActorLocation _pawn) (Transformation|GetActorLocation _grapplinghookattach))) (Math|Vector|DotProduct (- (Transformation|GetActorLocation _pawn) (Transformation|GetActorLocation _grapplinghookattach)) (Transformation|GetVelocity _pawn))) -2.0) (Variables|Settings|GetSwingMultiplier)) false false)
    (Character|LaunchCharacter _ascharacter (* (Math|Vector|GetUnitDirection(Vector) (Transformation|GetActorLocation _pawn) (Transformation|GetActorLocation _grapplinghookattach)) (Variables|Settings|GetPullMultiplier)) false false)))

(event EventBeginPlay
  ;[1 1 1] Enable Event Tick
  ; (For some reason it is disabled by default for custom items)
  (Actor|Tick|SetActorTickEnabled true)
  (CallFunction|Test))

(fn ConstructionScript)

(fn CanbeGrappeled?
  (params (Grappling%20player :type Player%20State%20Object%20Reference))
  (bind _pawn (Class|PavlovCustomItem|GetOwningPawn))
  (if (and (Utilities|IsValid _pawn) (!= Grappling%20player (Variables|/Script/Engine.Pawn|GetPlayerState _pawn)))
    (return true)
    (else
      (return false))))