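; BP_FloatingCube is an example-map cube that spins in place with a randomized speed and size.
; The construction script disables actor tick and gives the RotatingMovement component random speeds on two axes, leaving the third at zero.
; Spin speeds and the stepped uniform cube scale come from the Seed stream, while spin directions use unseeded RandomBool, so they are not reproducible from the seed.
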(fn ConstructionScript
  (bind _seed (Variables|Settings|GetSeed))
  (bind _returnvalue (Math|Random|RandomFloatinRangefromStream 3e+01 9e+01 _seed))
  (bind _returnvalue_2 (Math|Random|RandomFloatinRangefromStream 3e+01 9e+01 _seed))
  (Actor|Tick|SetActorTickEnabled false)
  (Variables|/Script/Engine.RotatingMovementComponent|SetRotationRate (Variables|Default|GetRotatingMovement) (Math|Rotator|MakeRotator 0.0 (select (Math|Random|RandomBool) _returnvalue_2 (* _returnvalue_2 -1.0)) (select (Math|Random|RandomBool) _returnvalue (* _returnvalue -1.0))))
  (Transformation|SetRelativeScale3D (Variables|Default|GetCube) (Math|Conversions|ToVector(Float) (* (Math|Random|RandomIntegerinRangefromStream 1 4 (Variables|Settings|GetSeed)) 0.5))))