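; MovingPlatform is an example map platform whose cube shuttles endlessly between a start and an end position.
; On BeginPlay a FlipFlop alternates playing and reversing the Movement timeline, which lerps the cube between the StartPos and EndPos world locations without sweep.
; Each time the timeline finishes, a MoveDelay pause runs before the FlipFlop fires again, creating a ping-pong loop.
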(event EventBeginPlay
  (Utilities|FlowControl|FlipFlop :!label _label
    (:A
      (bind _newtrack_0 (Timeline|Movement Play)
        (:Update
          (Transformation|SetWorldLocation (Variables|Default|GetCube) (Math|Vector|Lerp(Vector) (Transformation|GetWorldLocation (Variables|Default|GetStartPos)) (Transformation|GetWorldLocation (Variables|Default|GetEndPos)) _newtrack_0) false false))
        (:Finished
          (Utilities|FlowControl|Delay (Variables|Default|GetMoveDelay))
          (goto _label))))
    (:B
      (Timeline|Movement Reverse))))

(fn ConstructionScript)